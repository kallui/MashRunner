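; AIC_Runner is an AI controller that drives a possessed BP_Runner by simulating alternating left and right power inputs.
; On possession it caches the pawn as its runner.
; A non-looping timer starts on BeginPlay and re-arms after each simulated input with a new short random delay, so a FlipFlop alternates sides at a slightly irregular, rapid cadence.
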(event Custom|SimulateInput
  (Utilities|FlowControl|FlipFlop
    (:A
      (Default|SimulatePowerLeft (Variables|Default|GetOwningRunner)))
    (:B
      (Default|SimulatePowerRight (Variables|Default|GetOwningRunner))))
  (Utilities|Time|SetTimerbyEvent (EventDispatchers|CreateEvent :!event Custom|SimulateInput) (Math|Random|RandomFloatinRange 0.08 0.11)))

(event EventBeginPlay
  (Utilities|Time|SetTimerbyEvent (EventDispatchers|CreateEvent :!event Custom|SimulateInput) (Math|Random|RandomFloatinRange 0.08 0.11)))

(event EventPossess
  (params (PossessedPawn :type Pawn%20Object%20Reference))
  (bind _asbp_runner (Utilities|Casting|CastToBP_Runner PossessedPawn))
  (Variables|Default|SetOwningRunner _asbp_runner))

(fn ConstructionScript)