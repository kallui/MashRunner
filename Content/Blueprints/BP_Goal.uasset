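; BP_Goal is the finish line actor for the runner game, ending the race when a BP_Runner reaches it.
; On BeginPlay it caches the GM_Runner game mode.
; A box overlap with a runner fires once, swapping the Paper2D sprite to a ripped goal image and passing a player index to the game mode's HandleRaceOver.
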(event OnComponentBeginOverlap(Box)
  (params (OverlappedComponent :type Primitive%20Component%20Object%20Reference) (OtherActor :type Actor%20Object%20Reference) (OtherComp :type Primitive%20Component%20Object%20Reference) (OtherBodyIndex :type Integer) (bFromSweep :type Boolean) (SweepResult :type Hit%20Result%20Structure%20%28by%20ref%29))
  (Utilities|Casting|CastToBP_Runner OtherActor)
  (Utilities|FlowControl|DoOnce false
    (:Completed
      (CallFunction|UpdateGoalSprite)
      (Default|HandleRaceOver (Variables|Default|GetGameMode) (Variables|Default|GetPlayer%20Index)))))

(event EventBeginPlay
  (bind _asgm_runner (Utilities|Casting|CastToGM_Runner (Game|GetGameMode)))
  (Variables|Default|SetGameMode _asgm_runner))

(fn ConstructionScript)

(fn UpdateGoalSprite
  (Rendering|Components|Sprite|SetSprite (Variables|Default|GetPaperSprite) "/Game/PaperAssets/Goal/T_Goal_Ripped_Sprite.T_Goal_Ripped_Sprite"))